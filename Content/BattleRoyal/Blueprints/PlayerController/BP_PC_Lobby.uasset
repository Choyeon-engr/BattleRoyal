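; Lobby player controller for the BattleRoyal game that presents the menu and starts the trip into a match.
; On BeginPlay it plays music, views through the camera actor tagged LobbyCamera, and shows BP_UI_Lobby with UI-only input and a visible cursor.
; Its Play event takes an IP address and opens the intermediate Load level, passing the address as the NextLevel option rather than connecting directly.
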(event `self.ReceiveBeginPlay`
  (`GameplayStatics.PlaySound2D` "/Game/FantasyOrchestral/cues/MagicalFantasy.MagicalFantasy" 1.0 1.0 0.0 null null)
  (bind _outactors (`GameplayStatics.GetAllActorsWithTag` "LobbyCamera"))
  (bind _ascamera_actor (cast `CameraActor` (`|GetArrayItem` _outactors)))
  (`self.SetViewTargetWithBlend` _ascamera_actor)
  (bind _returnvalue (`|CreateWidget` "/Game/BattleRoyal/Blueprints/UI/BP_UI_Lobby.BP_UI_Lobby_C" self))
  (`/Engine/EditorBlueprintResources/StandardMacros.IsValid` _returnvalue
    (:`Is Valid`
      (`UserWidget.AddToViewport` _returnvalue 0)
      (`WidgetBlueprintLibrary.SetInputMode_UIOnlyEx` self _returnvalue)
      (set `self.bShowMouseCursor` true))))

(event `Play`
  (params (IpAddress :type String))
  (`GameplayStatics.OpenLevel` "Load" true (`KismetStringLibrary.Concat_StrStr` "NextLevel=" IpAddress)))

(fn `UserConstructionScript`)