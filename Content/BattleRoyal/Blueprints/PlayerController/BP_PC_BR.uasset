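; Battle royale player controller that manages a player's screen UI and the pawn swaps for riding a vehicle and dropping from it.
; On remote instances it creates a client message widget, also used for blood-screen flashes, and it shows death or winner results plus a hold-to-view world map.
; BoardVehicle replaces the pawn with a passenger attached to the vehicle.
; A one-time Descent replaces that with a descending Wraith character at the same location.
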(event `self.ReceiveBeginPlay`
  (`/Engine/EditorBlueprintResources/ActorMacros.Switch Has Authority`
    (:`Remote`
      (bind _asbrgame_state (cast `BRGameState` (`GameplayStatics.GetGameState`)))
      (bind _returnvalue (`|CreateWidget` "/Game/BattleRoyal/Blueprints/UI/BP_UI_ClientMessage.BP_UI_ClientMessage_C" self self _asbrgame_state))
      (bind _output_get (set `self.ClientMessageWidget` _returnvalue))
      (`UserWidget.AddToViewport` _output_get 0))))

(event `self.MessageToClient`
  (params (Message :type String))
  (set `self.Message` Message))

(event `self.DeathResult`
  (params (Rank :type Integer))
  (bind _returnvalue (`|CreateWidget` "/Game/BattleRoyal/Blueprints/UI/BP_UI_Result.BP_UI_Result_C" self "Let's play once again!" (`KismetStringLibrary.Concat_StrStr` "#" (`KismetStringLibrary.Conv_IntToString` Rank))))
  (`UserWidget.AddToViewport` _returnvalue 0))

(event `self.WinnerResult`
  (bind _returnvalue (`|CreateWidget` "/Game/BattleRoyal/Blueprints/UI/BP_UI_Result.BP_UI_Result_C" self "You win!" "#1"))
  (`UserWidget.AddToViewport` _returnvalue 0))

(event `self.BoardVehicle`
  (params (Vehicle :type "Actor Object Reference"))
  (`self.K2_DestroyActor` (`self.K2_GetPawn`))
  (bind _returnvalue (`|SpawnActorFromClass` "/Game/BattleRoyal/Blueprints/Character/BP_Passenger.BP_Passenger_C" (`self.GetTransform` Vehicle) "AlwaysSpawn" "OverrideRootScale" self null))
  (`self.Possess` _returnvalue)
  (`self.K2_AttachToActor` _returnvalue Vehicle "None" "SnapToTarget" "SnapToTarget" "SnapToTarget" false))

(event `Descent`
  (if (not (`self.bDescent`))
    (set `self.bDescent` true)
    (bind _returnvalue (`|SpawnActorFromClass` "/Game/BattleRoyal/Blueprints/Character/WraithPlayerCharacter.WraithPlayerCharacter_C" (`KismetMathLibrary.MakeTransform` (`self.K2_GetActorLocation` (`self.K2_GetPawn`))) "AlwaysSpawn" "OverrideRootScale" self null))
    (`self.K2_DestroyActor` (`self.K2_GetPawn`))
    (`self.Possess` _returnvalue)
    (set `BRCharacter.bDescent` true _returnvalue)))

(event `InputAction|WorldMap`
  (params (Key :type "Key Structure"))
  (bind _worldmapwidget (`self.WorldMapWidget`))
  (:`Pressed`
    (`/Engine/EditorBlueprintResources/StandardMacros.IsValid` _worldmapwidget
      (:`Is Valid`
        (`UserWidget.AddToViewport` _worldmapwidget 0))
      (:`Is Not Valid`
        (bind _returnvalue (`|CreateWidget` "/Game/BattleRoyal/Blueprints/UI/BP_UI_WorldMap.BP_UI_WorldMap_C" self self))
        (bind _output_get (set `self.WorldMapWidget` _returnvalue))
        (`UserWidget.AddToViewport` _output_get 0))))
  (:`Released`
    (`Widget.RemoveFromParent` (`self.WorldMapWidget`))))

(event `self.PrintBloodScreen`
  (bind _clientmessagewidget (`self.ClientMessageWidget`))
  (`/Engine/EditorBlueprintResources/StandardMacros.IsValid` _clientmessagewidget
    (:`Is Valid`
      (`UserWidget.PlayAnimation` _clientmessagewidget (`/Game/BattleRoyal/Blueprints/UI/BP_UI_ClientMessage.BloodAnim` _clientmessagewidget) 0.0 1 "Forward" 1.0 false))))

(fn `UserConstructionScript`)