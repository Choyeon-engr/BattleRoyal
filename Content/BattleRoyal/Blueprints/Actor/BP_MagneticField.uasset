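; BP_MagneticField is the actor that displays the battle royale's current circle, the magnetic field, in the world.
; Every Tick it casts the GameState to BRGameState and copies the circle's visibility and location onto itself.
; It scales X and Y from the circle radius divided by 50, with a large fixed Z scale for height.
; It only mirrors GameState values, with no circle or overlap logic of its own.
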(event `self.ReceiveTick`
  (params (DeltaSeconds :type "Float (single-precision)"))
  (bind _asbrgame_state (cast `BRGameState` (`GameplayStatics.GetGameState`)))
  (`SceneComponent.SetVisibility` (`self.MagneticField`) (`BRGameState.bVisibleCurCircle` _asbrgame_state) true)
  (`self.K2_SetActorLocation` (`BRGameState.CurCircleLoc` _asbrgame_state) false true)
  (bind _returnvalue (/ (`BRGameState.CurCircleRadius` _asbrgame_state) 50.0))
  (`self.SetActorScale3D` (`KismetMathLibrary.MakeVector` _returnvalue _returnvalue 1000.0)))

(fn `UserConstructionScript`)