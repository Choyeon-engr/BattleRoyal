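; BP_C130 is the transport plane actor for the battle royale mode that carries the match toward the drop.
; Four propellers spin locally every tick, while only the authority moves the plane forward at constant speed.
; Once it travels a set distance from its spawn point, it calls DescentAll on BP_GM_BR and destroys itself after a short delay.
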(event `self.ReceiveBeginPlay`
  (set `self.StartLocation` (`self.K2_GetActorLocation`)))

(event `self.ReceiveTick`
  (params (DeltaSeconds :type "Float (single-precision)"))
  (`SceneComponent.K2_AddLocalRotation` (`self.Prop1`) (`KismetMathLibrary.MakeRotator` 0.0 (* DeltaSeconds -720.0)) false false)
  (`SceneComponent.K2_AddLocalRotation` (`self.Prop2`) (`KismetMathLibrary.MakeRotator` 0.0 (* DeltaSeconds -720.0)) false false)
  (`SceneComponent.K2_AddLocalRotation` (`self.Prop3`) (`KismetMathLibrary.MakeRotator` 0.0 (* DeltaSeconds -720.0)) false false)
  (`SceneComponent.K2_AddLocalRotation` (`self.Prop4`) (`KismetMathLibrary.MakeRotator` 0.0 (* DeltaSeconds -720.0)) false false)
  (`/Engine/EditorBlueprintResources/ActorMacros.Switch Has Authority`
    (:`Authority`
      (`self.K2_AddActorLocalOffset` (`KismetMathLibrary.MakeVector` (* DeltaSeconds 3000.0)))
      (if (> (`KismetMathLibrary.VSize` (- (`self.K2_GetActorLocation`) (`self.StartLocation`))) 30000.0)
        (bind _asbp_gm_br (cast `/Game/BattleRoyal/Blueprints/GameMode/BP_GM_BR` (`GameplayStatics.GetGameMode`)))
        (`/Game/BattleRoyal/Blueprints/GameMode/BP_GM_BR.DescentAll` _asbp_gm_br)
        (`KismetSystemLibrary.Delay` 3.0)
        (`self.K2_DestroyActor`)))))

(fn `UserConstructionScript`)