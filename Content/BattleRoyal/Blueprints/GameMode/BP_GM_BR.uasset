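; Battle royale game mode that handles the drop plane and forced player descent.
; SpawnVehicle always spawns a BP_C130 at a fixed high-altitude, angled transform and stores it as Vehicle.
; DescentAll loops over AliveClients and calls Descent on each valid BP_PC_BR controller that has not already descended.
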(event `self.SpawnVehicle`
  (bind _returnvalue (`|SpawnActorFromClass` "/Game/BattleRoyal/Blueprints/Actor/BP_C130.BP_C130_C" (`KismetMathLibrary.MakeTransform` (-10000.0 10000.0 20000.0) (struct :`Yaw` -45.0)) "AlwaysSpawn" "OverrideRootScale" null null))
  (set `self.Vehicle` _returnvalue))

(event `DescentAll`
  (for _array_element (`self.AliveClients`)
    (bind _asbp_pc_br (cast `/Game/BattleRoyal/Blueprints/PlayerController/BP_PC_BR` _array_element))
    (`/Engine/EditorBlueprintResources/StandardMacros.IsValid` _asbp_pc_br
      (:`Is Valid`
        (if (not (`BRPlayerController.bDescent` _asbp_pc_br))
          (`/Game/BattleRoyal/Blueprints/PlayerController/BP_PC_BR.Descent` _asbp_pc_br))))))

(fn `UserConstructionScript`)