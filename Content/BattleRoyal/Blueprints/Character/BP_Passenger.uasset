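; BP_Passenger is the battle royale pawn a player controls as a passenger before descending.
; On BeginPlay, non-authority instances set the interaction widget prompt to "Descent".
; Turn and LookUp axes drive controller yaw and pitch, allowing the passenger only to look around.
; Pressing Interaction calls Descent on BP_PC_BR, leaving the descent logic to the player controller.
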(event `self.ReceiveBeginPlay`
  (`/Engine/EditorBlueprintResources/ActorMacros.Switch Has Authority`
    (:`Remote`
      (bind _asbp_ui_interaction (cast `/Game/BattleRoyal/Blueprints/UI/BP_UI_Interaction` (`WidgetComponent.GetUserWidgetObject` (`self.Widget`))))
      (set `/Game/BattleRoyal/Blueprints/UI/BP_UI_Interaction.Interaction` "Descent" _asbp_ui_interaction))))

(event `InputAxis|Turn`
  (params (AxisValue :type "Float (single-precision)"))
  (`self.AddControllerYawInput` AxisValue))

(event `InputAxis|LookUp`
  (params (AxisValue :type "Float (single-precision)"))
  (`self.AddControllerPitchInput` AxisValue))

(event `InputAction|Interaction`
  (params (Key :type "Key Structure"))
  (:`Pressed`
    (bind _asbp_pc_br (cast `/Game/BattleRoyal/Blueprints/PlayerController/BP_PC_BR` (`self.GetController`)))
    (`/Game/BattleRoyal/Blueprints/PlayerController/BP_PC_BR.Descent` _asbp_pc_br)))

(fn `UserConstructionScript`)